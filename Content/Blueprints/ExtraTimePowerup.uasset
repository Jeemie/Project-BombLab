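; ExtraTimePowerup is a spinning pickup that adds time to the game mode's timer when a ThirdPersonCharacter overlaps it.
; It notifies the player's HUD first, then, only if a BP_Bomb exists, extends the BP_PBGGameMode timer, plays a ticking sound and destroys itself.
; The bomb lookup serves only as a gate, as its AddTime call is disconnected.
; A self-restarting timeline drives the yaw spin.
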(event `self.ReceiveActorBeginOverlap`
  (params (OtherActor :type "Actor Object Reference"))
  (bind _asthird_person_character (cast `/Game/Blueprints/ThirdPerson_WallJump_Character` OtherActor))
  ;[1 1 1] Display in HUD
  (`/Game/Blueprints/PlayerHUD.GetPowerup` (`/Game/Blueprints/ThirdPerson_WallJump_Character.PlayerHUD` _asthird_person_character) 3)
  ;[1 1 1] Get reference to bomb
  (bind _outactors (`GameplayStatics.GetAllActorsOfClass` "/Game/Blueprints/BP_Bomb.BP_Bomb_C"))
  (if (> (`KismetArrayLibrary.Array_Length` _outactors) 0)
    (bind _asbp_pbggame_mode (cast `/Game/Blueprints/BP_PBGGameMode` (`GameplayStatics.GetGameMode`)))
    (set `/Game/Blueprints/BP_PBGGameMode.Timer` (+ (`/Game/Blueprints/BP_PBGGameMode.Timer` _asbp_pbggame_mode) 20.0) _asbp_pbggame_mode)
    ;[1 1 1] Play sound effect
    (`GameplayStatics.PlaySoundAtLocation` "/Game/Sounds/ClockTicks.ClockTicks" (`self.K2_GetActorLocation`))
    (`self.K2_DestroyActor`)))

(event `self.ReceiveBeginPlay`
  (bind (_direction _rotation) (`Timeline|Rotation` :!via `PlayFromStart` :!label _label)
    (:`Update`
      (`self.K2_SetActorRotation` (`KismetMathLibrary.MakeRotator` 0.0 0.0 _rotation)))
    (:`Finished`
      (`self.Restart`))))

(event `Restart`
  (goto _label :!via `PlayFromStart`))

(fn `UserConstructionScript`)