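; BP_PBGGameMode is a game mode that runs a countdown and shows a game over screen when time runs out.
; BeginPlay adds the Timer widget to the viewport and starts a looping one-second timer that decrements the Timer variable.
; At zero or below it prints a message and adds a GameOver widget.
; The `>= 0` guard lets this repeat once after reaching exactly zero, and the looping timer is never cleared.
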(event `self.ReceiveBeginPlay`
  (bind _returnvalue (`|CreateWidget` "/Game/Blueprints/Timer.Timer_C"))
  (`UserWidget.AddToViewport` _returnvalue 0)
  (`KismetSystemLibrary.K2_SetTimerDelegate` (delegate `TimeCounter`) 1.0 true))

(event `TimeCounter`
  (if (>= (`self.Timer`) 0.0)
    (bind _output_get (set `self.Timer` (- (`self.Timer`) 1.0)))
    (if (<= _output_get 0.0)
      (`KismetSystemLibrary.PrintString` "Time runs out!")
      (bind _returnvalue (`|CreateWidget` "/Game/Blueprints/GameOver.GameOver_C"))
      (`UserWidget.AddToViewport` _returnvalue 0))))

(fn `UserConstructionScript`)