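; A double-jump powerup pickup that spins in place until the player touches it.
; On overlap with a ThirdPersonCharacter it notifies the player HUD, sets the character's double-jump count, plays a wing-flap sound at its location and destroys itself.
; A timeline started on BeginPlay drives the yaw rotation and restarts itself through a custom event each time it finishes.
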(event `self.ReceiveActorBeginOverlap`
  (params (OtherActor :type "Actor Object Reference"))
  (bind _asthird_person_character (cast `/Game/Blueprints/ThirdPerson_WallJump_Character` OtherActor))
  ;[1 1 1] Display in HUD
  (`/Game/Blueprints/PlayerHUD.GetPowerup` (`/Game/Blueprints/ThirdPerson_WallJump_Character.PlayerHUD` _asthird_person_character) 2)
  ;[1 1 1] Give player 3 double jumps
  (set `/Game/Blueprints/ThirdPerson_WallJump_Character.DoubleJumpCount` 3 _asthird_person_character)
  ;[1 1 1] Play sound effect
  (`GameplayStatics.PlaySoundAtLocation` "/Game/Sounds/WingFlap.WingFlap" (`self.K2_GetActorLocation`))
  (`self.K2_DestroyActor`))

(event `self.ReceiveBeginPlay`
  (bind (_direction _rotation) (`Timeline|Rotation` :!via `PlayFromStart` :!label _label)
    (:`Update`
      (`self.K2_SetActorRotation` (`KismetMathLibrary.MakeRotator` 0.0 0.0 _rotation)))
    (:`Finished`
      (`self.Restart`))))

(event `Restart`
  (goto _label :!via `PlayFromStart`))

(fn `UserConstructionScript`)