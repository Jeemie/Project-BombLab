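; Crate manager that spawns BP_Crate actors at BP_CrateSpawnpoint locations in the level.
; BeginPlay seeds randomness, resets the drop table, then fills ten randomly chosen spawnpoints.
; SpawnBox adds one crate from the unoccupied spawnpoints, but re-rolls its random index at each step rather than caching one pick.
; Crates receive references to their spawnpoint and manager, and spawnpoints track occupancy and their crate.
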(event `self.ReceiveBeginPlay`
  (`self.initRandomSeed`)
  (`self.resetDropTable`)
  (`self.Initial Spawn` 10))

(fn `Spawn Box`
  (locals (AvailableSpawnpoints :type "Array of /Game/Blueprints/BP_CrateSpawnpoint Object Reference"))
  (bind _availablespawnpoints (`local.AvailableSpawnpoints`))
  (bind _availablespawnpoints_2 (`local.AvailableSpawnpoints`))
  (bind _output (`|GetArrayItem` _availablespawnpoints_2 (`KismetMathLibrary.RandomIntegerInRange` 0 (- (`KismetArrayLibrary.Array_Length` _availablespawnpoints_2) 1))))
  (bind _outactors (`GameplayStatics.GetAllActorsOfClass` "/Game/Blueprints/BP_CrateSpawnpoint.BP_CrateSpawnpoint_C"))
  ;[1 1 1] Get spawnpoints with no box
  (for _array_element _outactors
    (if (not (`/Game/Blueprints/BP_CrateSpawnpoint.IsSpawned` _array_element))
      (`KismetArrayLibrary.Array_Add` _availablespawnpoints _array_element)))
  ;[1 1 1] Check if any spawnpoints were found
  (if (> (`KismetArrayLibrary.Array_Length` _availablespawnpoints) 0)
    ;[1 1 1] Generate box
    (set `/Game/Blueprints/BP_CrateSpawnpoint.IsSpawned` true _output)
    (bind _returnvalue (`|SpawnActorFromClass` "/Game/Blueprints/BP_Crate.BP_Crate_C" (`self.GetTransform` _output) "AdjustIfPossibleButAlwaysSpawn" "OverrideRootScale" null null))
    (`self.K2_SetActorLocation` _returnvalue (`self.K2_GetActorLocation` _output) false true)
    (set `/Game/Blueprints/BP_Crate.SpawnpointRef` _output _returnvalue)
    (set `/Game/Blueprints/BP_CrateSpawnpoint.CrateRef` _returnvalue _output)
    (set `/Game/Blueprints/BP_Crate.ManagerRef` self _returnvalue)))

(fn `UserConstructionScript`)