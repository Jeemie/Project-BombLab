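; BP_Bomb is the bomb objective that the player defuses in several phases to win the game.
; On BeginPlay it finds the single ThirdPersonCharacter and seeds the GameMode's timer and phase count, the latter for the HUD.
; DefuseBomb requires the player nearby with a defuser, consumes it, adds time and decrements the phases.
; The last phase triggers the win and disables player input, while earlier ones reset the BP_CrateManager drop table.
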(event `self.ReceiveBeginPlay`
  ;[1 1 1] Get player reference
  (bind _outactors (`GameplayStatics.GetAllActorsOfClass` "/Game/Blueprints/ThirdPerson_WallJump_Character.ThirdPersonCharacter_C"))
  (if (== 1 (`KismetArrayLibrary.Array_Length` _outactors))
    (set `self.Player` (`|GetArrayItem` _outactors))
    ;[1 1 1] Setup bomb
    (bind _output_get (set `self.TimeRemaining` 120.0))
    (bind _asbp_pbggame_mode (cast `/Game/Blueprints/BP_PBGGameMode` (`GameplayStatics.GetGameMode`)))
    (set `/Game/Blueprints/BP_PBGGameMode.Timer` _output_get _asbp_pbggame_mode)
    (`self.SetActorTickEnabled` true)
    (bind _output_get_2 (set `self.PhasesLeft` 3))
    ;[1 1 1] Pass remaining phases to Gamemode (for HUD)
    (bind _asbp_pbggame_mode_2 (cast `/Game/Blueprints/BP_PBGGameMode` (`GameplayStatics.GetGameMode`)))
    (set `/Game/Blueprints/BP_PBGGameMode.Phases` _output_get_2 _asbp_pbggame_mode_2)))

(fn `Add Time`
  (params (ExtraTime :type "Float (double-precision)"))
  (set `self.TimeRemaining` (+ (`self.TimeRemaining`) ExtraTime)))

(fn `DefuseBomb`
  (bind _player (`self.Player`))
  ;[1 1 1] Is player close to bomb and has defuser?
  (if (and (>= 300.0 (`self.GetDistanceTo` _player)) (`/Game/Blueprints/ThirdPerson_WallJump_Character.bHasDefuser` _player))
    ;[1 1 1] Take defuser from player, add time and defuse phase
    (set `/Game/Blueprints/ThirdPerson_WallJump_Character.bHasDefuser` false (`self.Player`))
    (bind _asbp_pbggame_mode (cast `/Game/Blueprints/BP_PBGGameMode` (`GameplayStatics.GetGameMode`)))
    (set `/Game/Blueprints/BP_PBGGameMode.Timer` (+ (`/Game/Blueprints/BP_PBGGameMode.Timer` _asbp_pbggame_mode) 30.0) _asbp_pbggame_mode)
    ;[1 1 1] Decrement remaining phases and pass to Gamemode (for HUD)
    (bind _asbp_pbggame_mode_2 (cast `/Game/Blueprints/BP_PBGGameMode` (`GameplayStatics.GetGameMode`)))
    (bind _result (`/Engine/EditorBlueprintResources/StandardMacros.DecrementInt` (`self.PhasesLeft`))
      (:`  `
        (bind _output_get (set `/Game/Blueprints/BP_PBGGameMode.Phases` _result _asbp_pbggame_mode_2))
        ;[1 1 1] Win check
        (if (<= _output_get 0)
          ;[1 1 1] Disable bomb
          (`self.SetActorTickEnabled` false)
          ;[1 1 1] Play sound effect
          (`GameplayStatics.PlaySound2D` "/Game/Sounds/LevelUp.LevelUp")
          (set `/Game/Blueprints/ThirdPerson_WallJump_Character.wonGame` true (`self.Player`))
          (`self.DisableInput` (`self.Player`) (`GameplayStatics.GetPlayerController` 0))
          (else
            ;[1 1 1] Play sound effect
            (`GameplayStatics.PlaySound2D` "/Game/Sounds/StartDefusing.StartDefusing")
            ;[1 1 1] Reset drop Table
            (bind _outactors (`GameplayStatics.GetAllActorsOfClass` "/Game/Blueprints/BP_CrateManager.BP_CrateManager_C"))
            (if (> (`KismetArrayLibrary.Array_Length` _outactors) 0)
              (`CrateManager.resetDropTable` (`|GetArrayItem` _outactors)))))))))

(fn `UserConstructionScript`)