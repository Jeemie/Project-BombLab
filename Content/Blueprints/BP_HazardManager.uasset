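; Hazard manager actor that spawns BP_BombHazard at its own transform on a randomly varied countdown, paced by the main bomb's remaining phases.
; Tick runs the countdown while enabled, then checks the single BP_Bomb's PhasesLeft after each spawn, or every tick while disabled.
; Two phases left enables hazards, one shortens the spawn interval, and zero disables them.
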(event `self.ReceiveBeginPlay`
  (bind _spawnrate (`self.SpawnRate`))
  (set `self.Timer` (+ (* (`KismetMathLibrary.RandomFloatInRange` -0.2 0.2) _spawnrate) _spawnrate)))

(event `self.ReceiveTick`
  (params (DeltaSeconds :type "Float (single-precision)"))
  (if (`self.Enabled`)
    ;[1 1 1] Tick down timer
    (bind _output_get (set `self.Timer` (- (`self.Timer`) DeltaSeconds)))
    ;[1 1 1] If timer ran out...
    (if (<= _output_get 0.0)
      ;[1 1 1] Spawn bomb
      (`|SpawnActorFromClass` "/Game/Blueprints/BP_BombHazard.BP_BombHazard_C" (`self.GetTransform` self) "Undefined" "OverrideRootScale" null null)
      ;[1 1 1] Safety check
      (bind _outactors (`GameplayStatics.GetAllActorsOfClass` "/Game/Blueprints/BP_Bomb.BP_Bomb_C" :!label _label))
      (if (== (`KismetArrayLibrary.Array_Length` _outactors) 1)
        ;[1 1 1] How many phases are left?
        (switch `int` (`/Game/Blueprints/BP_Bomb.PhasesLeft` (`|GetArrayItem` _outactors))
          (:`0`
            ;[1 1 1] Disable hazards
            (set `self.Enabled` false))
          (:`1`
            (bind _output_get_2 (set `self.SpawnRate` 1.4))
            ;[1 1 1] Reset timer (with slight variation
            (set `self.Timer` (+ (* (`KismetMathLibrary.RandomFloatInRange` -0.1 0.1) _output_get_2) _output_get_2)))
          (:`2`
            ;[1 1 1] Enable hazards
            (set `self.Enabled` true)
            (bind _output_get_3 (set `self.SpawnRate` 3.5))
            ;[1 1 1] Reset timer (with slight variation
            (set `self.Timer` (+ (* (`KismetMathLibrary.RandomFloatInRange` -0.1 0.1) _output_get_3) _output_get_3))))))
    (else
      (goto _label))))

(fn `UserConstructionScript`)