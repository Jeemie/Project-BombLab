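; Falling bomb hazard that targets the ThirdPersonCharacter.
; On BeginPlay it teleports high above a random point around the player, biased ahead of their facing.
; Each Tick it descends, drifts toward the player by a frame-rate-dependent step, and line-traces down to place a spinning target sprite on the floor.
; The first overlap detonates it, damaging a nearby player who hasn't won, playing sound and particles, then destroying itself after a delay.
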(event `self.ReceiveBeginPlay`
  (bind _returnvalue (`KismetMathLibrary.RandomFloatInRange` 0.0 360.0))
  (bind _returnvalue_2 (`KismetMathLibrary.RandomFloatInRange` -3000.0 3000.0))
  (bind _outactors (`GameplayStatics.GetAllActorsOfClass` "/Game/Blueprints/ThirdPerson_WallJump_Character.ThirdPersonCharacter_C"))
  ;[1 1 1] Get character
  (if (== (`KismetArrayLibrary.Array_Length` _outactors) 1)
    (bind _output (`|GetArrayItem` _outactors))
    ;[1 1 1] Spawn bomb
    (`self.K2_TeleportTo` (+ (`KismetMathLibrary.MakeVector` (* (`KismetMathLibrary.DegSin` _returnvalue) _returnvalue_2) (* _returnvalue_2 (`KismetMathLibrary.DegCos` _returnvalue)) 1200.0) (`self.K2_GetActorLocation` _output) (* (`SceneComponent.GetForwardVector` (`Character.CapsuleComponent` _output)) 500)))
    (`self.SetActorScale3D` (17.0 17.0 17.0))))

(event `self.ReceiveTick`
  (params (DeltaSeconds :type "Float (single-precision)"))
  ;[1 1 1] Move slighlty towards character
  (bind _outactors (`GameplayStatics.GetAllActorsOfClass` "/Game/Blueprints/ThirdPerson_WallJump_Character.ThirdPersonCharacter_C"))
  (bind _returnvalue (+ (* (`KismetMathLibrary.GetDirectionUnitVector` (`KismetMathLibrary.MakeVector` (.x (`SceneComponent.K2_GetComponentLocation` (`self.SkeletalMesh`))) (.y (`SceneComponent.K2_GetComponentLocation` (`self.SkeletalMesh`)))) (`KismetMathLibrary.MakeVector` (.x (`self.K2_GetActorLocation` (`|GetArrayItem` _outactors))) (.y (`self.K2_GetActorLocation` (`|GetArrayItem` _outactors))))) 3.0) (`SceneComponent.K2_GetComponentLocation` (`self.SkeletalMesh`)) (`KismetMathLibrary.MakeVector` 0.0 0.0 (* DeltaSeconds -260.0))))
  ;[1 1 1] Final movement
  (`SceneComponent.K2_SetWorldLocation` (`self.SkeletalMesh`) _returnvalue true false)
  ;[1 1 1] Detect floor
  (bind _outhit (`KismetSystemLibrary.LineTraceSingle` _returnvalue (- _returnvalue (0.0 0.0 3000.0)) "TraceTypeQuery3"))
  ;[1 1 1] Draw target sprite slightly above floor
  (`SceneComponent.K2_SetWorldLocation` (`self.PaperSprite`) (+ (`.Location` (`GameplayStatics.BreakHitResult` _outhit)) (0.0 0.0 15.0)) false true)
  ;[1 1 1] Slightly rotate sprite
  (`SceneComponent.K2_AddRelativeRotation` (`self.PaperSprite`) (`KismetMathLibrary.MakeRotator` 0.0 0.0 (* DeltaSeconds 50.0)) false false))

(event `self.ReceiveActorBeginOverlap`
  (params (OtherActor :type "Actor Object Reference"))
  ;[1 1 1] Don't explode twice in a row
  (if (not (`self.bDetonated`))
    (set `self.bDetonated` true)
    ;[1 1 1] If player is within blast radius...
    (bind _outactors (`GameplayStatics.GetAllActorsOfClass` "/Game/Blueprints/ThirdPerson_WallJump_Character.ThirdPersonCharacter_C"))
    (bind _output (`|GetArrayItem` _outactors))
    (if (<= (`self.GetDistanceTo` _output) 400.0)
      (if (not (`/Game/Blueprints/ThirdPerson_WallJump_Character.wonGame` _output))
        ;[1 1 1] Deal damage to player
        (`/Game/Blueprints/ThirdPerson_WallJump_Character.Damage` _output 15.0 (`KismetMathLibrary.GetDirectionUnitVector` (`self.K2_GetActorLocation` self) (`self.K2_GetActorLocation` _output)))))
    ;[1 1 1] Play sound effect
    (`GameplayStatics.PlaySoundAtLocation` "/Game/Sounds/Explosion.Explosion" (0.0 0.0 0.0) (struct) (`KismetMathLibrary.RandomFloatInRange` 0.35 0.5) (`KismetMathLibrary.RandomFloatInRange` 0.8 1.3))
    ;[1 1 1] Visual effects
    (`SceneComponent.SetVisibility` (`self.SkeletalMesh`) false false)
    (`SceneComponent.SetVisibility` (`self.PaperSprite`) false false)
    (`ActorComponent.Activate` (`self.ParticleSystem`) false)
    ;[1 1 1] Delete actor
    (`KismetSystemLibrary.Delay` 2.6)
    (`self.K2_DestroyActor`)))

(fn `UserConstructionScript`)