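; Health pickup that heals a ThirdPersonCharacter on overlap and spins in place while waiting.
; On overlap it notifies the player's HUD, updates health, plays a heal sound at its location and destroys itself.
; The cap is checked before the fixed increment is added, so health can end above the maximum.
; A timeline started on BeginPlay drives the yaw and restarts itself when finished for continuous rotation.
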(event `self.ReceiveActorBeginOverlap`
  (params (OtherActor :type "Actor Object Reference"))
  (bind _asthird_person_character (cast `/Game/Blueprints/ThirdPerson_WallJump_Character` OtherActor))
  ;[1 1 1] Display in HUD
  (`/Game/Blueprints/PlayerHUD.GetPowerup` (`/Game/Blueprints/ThirdPerson_WallJump_Character.PlayerHUD` _asthird_person_character) 1)
  (bind _health (`/Game/Blueprints/ThirdPerson_WallJump_Character.Health` _asthird_person_character))
  ;[1 1 1] Check that health won't go over 100%
  (if (>= _health 100.0)
    ;[1 1 1] Set new health
    (set `/Game/Blueprints/ThirdPerson_WallJump_Character.Health` 100.0 _asthird_person_character)
    (else
      (set `/Game/Blueprints/ThirdPerson_WallJump_Character.Health` (+ _health 25.0) _asthird_person_character)))
  ;[1 1 1] Play sound effect
  (`GameplayStatics.PlaySoundAtLocation` "/Game/Sounds/RPG_Heal_Sound_Fx.RPG_Heal_Sound_Fx" (`self.K2_GetActorLocation`))
  (`self.K2_DestroyActor`))

(event `self.ReceiveBeginPlay`
  (bind (_direction _rotation) (`Timeline|Rotation` :!via `PlayFromStart` :!label _label)
    (:`Update`
      (`self.K2_SetActorRotation` (`KismetMathLibrary.MakeRotator` 0.0 0.0 _rotation)))
    (:`Finished`
      (`self.Restart`))))

(event `Restart`
  (goto _label :!via `PlayFromStart`))

(fn `UserConstructionScript`)